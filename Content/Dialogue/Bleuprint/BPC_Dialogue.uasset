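; BPC_Dialogue is a component that plays dialogue lines through a WBP_Dialogue widget, created on BeginPlay.
; Each Speech call stores the passed dialogue struct, sends the current line's text, speaker name, sound and delay to the widget, then advances the index.
; Once the index reaches one past the line count, on the call after the last line, it resets the index, empties the struct and clears the widget text.
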(event Custom|Event%20Speech
  (params (SDialogues :type S%20Dialogue%20Structure))
  (Variables|Default|SetSDialogues SDialogues)
  (Default|EnventIncomingDialogue (Variables|Default|GetWidget%20Dialogue%20Ref) (Utilities|Array|Get(acopy) (.dialoguestext (Variables|Default|GetSDialogues)) (Variables|Default|GetCurrent%20Dialogue%20Index)) (.name (Variables|Default|GetSDialogues)) (Utilities|Array|Get(acopy) (.dialoguessound (Variables|Default|GetSDialogues)) (Variables|Default|GetCurrent%20Dialogue%20Index)) (.delay (Variables|Default|GetSDialogues)))
  (bind _result (Math|Integer|IncrementInt (Variables|Default|GetCurrent%20Dialogue%20Index))
    (:%20%20
      (if (>= _result (+ (Utilities|Array|Length (.dialoguestext (Variables|Default|GetSDialogues))) 1))
        (Variables|Default|SetCurrent%20Dialogue%20Index 0)
        (Variables|Default|SetSDialogues "")
        (Default|EventClearDialogueText (Variables|Default|GetWidget%20Dialogue%20Ref))))))

(event EventBeginPlay
  (bind _returnvalue (UserInterface|CreateWidget "/Game/Dialogue/Widget/WBP_Dialogue.WBP_Dialogue_C"))
  (Variables|Default|SetWidget%20Dialogue%20Ref _returnvalue))
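; BP_Interact is an interactable base in the Door props folder that accepts player input only from inside its front or back trigger.
; Each trigger opens and closes its own gate as the player overlaps it, and IntractionInput feeds both gates.
; An open gate calls InteractionFonction, empty here, if the player's LookActor is valid.
; IsFront is set true on back-trigger overlap and false on exit, for any actor.
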(event OnComponentBeginOverlap(InteractionFront)
  (params (OverlappedComponent :type Primitive%20Component%20Object%20Reference) (OtherActor :type Actor%20Object%20Reference) (OtherComp :type Primitive%20Component%20Object%20Reference) (OtherBodyIndex :type Integer) (bFromSweep :type Boolean) (SweepResult :type Hit%20Result%20Structure%20%28by%20ref%29))
  ;[1 1 1] Front Trigger
  (if (== OtherActor (Game|GetPlayerCharacter 0))
    (Utilities|FlowControl|Gate true) ; enters at Open
  ))

(event OnComponentBeginOverlap(InteractionBack)
  (params (OverlappedComponent :type Primitive%20Component%20Object%20Reference) (OtherActor :type Actor%20Object%20Reference) (OtherComp :type Primitive%20Component%20Object%20Reference) (OtherBodyIndex :type Integer) (bFromSweep :type Boolean) (SweepResult :type Hit%20Result%20Structure%20%28by%20ref%29))
  ;[1 1 1] Back Trigger
  (Variables|Default|SetIs%20Front%20?%20 true)
  (if (== OtherActor (Game|GetPlayerCharacter 0))
    (Utilities|FlowControl|Gate true) ; enters at Open
  ))

(event OnComponentEndOverlap(InteractionFront)
  (params (OverlappedComponent :type Primitive%20Component%20Object%20Reference) (OtherActor :type Actor%20Object%20Reference) (OtherComp :type Primitive%20Component%20Object%20Reference) (OtherBodyIndex :type Integer))
  ;[1 1 1] Front Trigger
  (if (== (Game|GetPlayerCharacter 0) OtherActor)
    (Utilities|FlowControl|Gate true) ; enters at Close
  ))

(event OnComponentEndOverlap(InteractionBack)
  (params (OverlappedComponent :type Primitive%20Component%20Object%20Reference) (OtherActor :type Actor%20Object%20Reference) (OtherComp :type Primitive%20Component%20Object%20Reference) (OtherBodyIndex :type Integer))
  ;[1 1 1] Back Trigger
  (Variables|Default|SetIs%20Front%20?%20 false)
  (if (== (Game|GetPlayerCharacter 0) OtherActor)
    (Utilities|FlowControl|Gate true) ; enters at Close
  ))

(event EventIntractionInput
  (Utilities|FlowControl|Sequence
    (:then_0
      ;[1 1 1] Front Trigger
      (Utilities|FlowControl|Gate true
        (:Exit
          (Variables|/Game/_GameManager/Player/Blueprints/BP_Player_Charachter.BP_Player_Charachter_C|GetLook%20Actor (.AsBP%20Player%20Charachter (Utilities|Casting|CastToBP_Player_Charachter (Game|GetPlayerCharacter 0)))
            (:then
              (CallFunction|InteractionFonction))
            (:else)))))
    (:then_1
      ;[1 1 1] Back Trigger
      (Utilities|FlowControl|Gate true
        (:Exit
          (Variables|/Game/_GameManager/Player/Blueprints/BP_Player_Charachter.BP_Player_Charachter_C|GetLook%20Actor (.AsBP%20Player%20Charachter (Utilities|Casting|CastToBP_Player_Charachter (Game|GetPlayerCharacter 0)))
            (:then
              (CallFunction|InteractionFonction))
            (:else)))))))

(fn ConstructionScript)

(fn InteractionFonction)
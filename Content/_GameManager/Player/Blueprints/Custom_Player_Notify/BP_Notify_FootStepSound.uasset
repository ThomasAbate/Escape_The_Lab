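; Animation notify that plays surface-dependent footstep sounds for the player.
; When fired, it line-traces 100 units straight down from the mesh owner's location on the Visibility channel and reads the hit's physical surface type.
; Wood and Tile surfaces play their wood or concrete sound cue at the impact point; other surfaces stay silent.
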(fn GetDefaultTriggerWeightThreshold)

(fn ReceivedNotify
  (params (MeshComp :type Skeletal%20Mesh%20Component%20Object%20Reference) (Animation :type Anim%20Sequence%20Base%20Object%20Reference) (EventReference :type Anim%20Notify%20Event%20Reference%20Structure%20%28by%20ref%29))
  (bind _returnvalue (Components|GetOwner MeshComp))
  (bind _returnvalue_2 (Transformation|GetActorLocation _returnvalue))
  (bind _outhit (Collision|LineTraceByChannel _returnvalue_2 (- _returnvalue_2 "0.000000,0.000000,100.000000") "TraceTypeQuery1" false 0 "None"))
  (if (.bBlockingHit (Collision|BreakHitResult _outhit))
    (switch Utilities|FlowControl|Switch|SwitchonEPhysicalSurface (Collision|GetSurfaceType _outhit)
      (:SurfaceType_Default
        _)
      (:SurfaceType1
        (Audio|PlaySoundatLocation "/Game/_GameManager/placeholder/Audio/FootStep/SC_footstep_wood.SC_footstep_wood" (.ImpactPoint (Collision|BreakHitResult _outhit)) "0, 0, 0" 1.0 1.0 0.0 0 0 0 0))
      (:SurfaceType2
        (Audio|PlaySoundatLocation "/Game/_GameManager/placeholder/Audio/FootStep/SC_footstep_on_concrete.SC_footstep_on_concrete" (.ImpactPoint (Collision|BreakHitResult _outhit)) "0, 0, 0" 1.0 1.0 0.0 0 0 0 0)))
    (return false)))
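; Player character Blueprint with push-to-talk voice chat, tuned jump gravity and autofocus depth of field.
; VOIP setup retries until PlayerState is valid, V toggles speaking, and ProxyChat's audio envelope maps logarithmically to MicValue.
; Falling starts with lighter gravity that increases at the jump apex, while a looping timer targets a camera sphere trace that sets focal distance.
; Tick holds test code printing traced jump height, its maximum and walk speed.
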(event OnAudioEnvelopeValue(ProxyChat)
  (params (EnvelopeValue :type Float%20%28single-precision%29))
  ;[0.05098 0.05098 0.05098] Spake in game
  (Variables|Mic|SetMic%20Value (Math|Float|MapRangeClamped (Math|Float|Log EnvelopeValue 1e+01) -2.7 -0.7 0.0 1.0)))

(event Custom|Event%20Blur%20Camera
  (bind _camera (Variables|Default|GetCamera))
  (bind _returnvalue (Transformation|GetWorldLocation _camera))
  ;[0.05098 0.05098 0.05098] Focus Camera
  (bind (_outhit _returnvalue_2) (Collision|SphereTraceByChannel _returnvalue (+ _returnvalue (* (Math|Vector|GetForwardVector _camera) (Variables|Camera|GetMax%20View%20Distance))) 1.0 "TraceTypeQuery1" false 0 "None"))
  (if _returnvalue_2
    (bind _output_get (Variables|Camera|SetFocus%20Location (Math|Vector|VectorLength (- (.Location (Collision|BreakHitResult _outhit)) (Transformation|GetWorldLocation (Variables|Default|GetCamera))))))
    (Variables|/Script/Engine.CameraComponent|SetPostProcessSettings (Variables|Default|GetCamera) (Utilities|Struct|MakePostProcessSettings 0.8 1e+02 _output_get))
    (else
      (Variables|/Script/Engine.CameraComponent|SetPostProcessSettings (Variables|Default|GetCamera) (Utilities|Struct|MakePostProcessSettings 0.8 1e+02 (/ (Variables|Camera|GetMax%20View%20Distance) 2.0))))))

(event Custom|Put%20Begin%20Play
  (bind _returnvalue (Game|GetPlayerState 0))
  ;[1 0 0] Voice Chat
  (bind _returnvalue_2 (AddComponent|AddVOIPTalker))
  (bind _output_get (Variables|Mic|SetMic_Ref _returnvalue_2))
  (Utilities|IsValid _returnvalue :!label _label
    (:Is%20Valid
      (Class|VOIPTalker|RegisterwithPlayerState _output_get _returnvalue)
      (Class|VOIPStatics|SetMicThreshold -1.0)
      (Variables|/Script/Engine.VOIPTalker|SetSettings (Variables|Mic|GetMic_Ref) (Utilities|Struct|MakeVoiceSettings (Variables|Collision|GetCapsuleComponent) "/Game/_GameManager/Player/Mic_Settings/Attenuation/ATT_Player.ATT_Player" 0))
      (if (Pawn|IsLocallyControlled)
        (Development|ExecuteConsoleCommand "OSS VoiceLoopback 1" 0)))
    (:Is%20Not%20Valid
      (Utilities|FlowControl|Delay 0.2)
      (goto _label))))

(event Custom|ApexReached
  ;[0.05098 0.05098 0.05098] Apex For Jump
  (Variables|/Script/Engine.CharacterMovementComponent|SetGravityScale (Variables|Character|GetCharacterMovement) 2.75))

(event EventOnMovementModeChanged
  (params (PrevMovementMode :type EMovementMode%20Enum :default "MOVE_None") (NewMovementMode :type EMovementMode%20Enum :default "MOVE_None") (PrevCustomMode :type Byte :default 0) (NewCustomMode :type Byte :default 0))
  (bind _charactermovement (Variables|Character|GetCharacterMovement))
  ;[0.05098 0.05098 0.05098] Apex For Jump
  (bind _output_get (Variables|/Script/Engine.CharacterMovementComponent|SetbNotifyApex _charactermovement (Utilities|Enum|Equal(Enum) NewMovementMode "MOVE_Falling")))
  (if _output_get
    (Variables|/Script/Engine.CharacterMovementComponent|SetGravityScale _charactermovement 1.75)
    (Character|BindEventtoOnReachedJumpApex (delegate Custom|ApexReached))
    (else
      (EventDispatchers|UnbindallEventsfromOnReachedJumpApex))))

(event EventBeginPlay
  ;[0.05098 0.05098 0.05098] Begin Player
  (Utilities|Time|SetTimerbyFunctionName 0 "Event Blur Camera" 0.2 true))

(event EventTick
  (params (DeltaSeconds :type Float%20%28single-precision%29))
  (bind _capsulecomponent (Variables|Collision|GetCapsuleComponent))
  (bind _returnvalue (Transformation|GetWorldLocation _capsulecomponent))
  ;[0.9844 0.9844 0.9844] Test Nodes
  (Utilities|FlowControl|Sequence
    (:then_0
      (bind _outhit (Collision|LineTraceByChannel _returnvalue (- _returnvalue "0.000000,0.000000,1000.000000") "TraceTypeQuery1" false 0 "ForDuration" true "(R=1.000000,G=0.000000,B=0.000000,A=1.000000)" "(R=0.000000,G=1.000000,B=0.000000,A=1.000000)" 0.2))
      (Utilities|FlowControl|Sequence
        (:then_0
          (Development|PrintString (Utilities|String|ToString(Float) (- (.Distance (Collision|BreakHitResult _outhit)) (stale _output_get_2))) true true "(R=0.000000,G=0.660000,B=1.000000,A=1.000000)" 0.0)
          (if (> (- (.Distance (Collision|BreakHitResult _outhit)) (Variables|Default|GetDefault%20Distance)) (Variables|Default|GetHigt%20Jump))
            (bind _output_get (Variables|Default|SetHigt%20Jump (- (.Distance (Collision|BreakHitResult _outhit)) (Variables|Default|GetDefault%20Distance)))))
          (Development|PrintString (Utilities|String|ToString(Float) _output_get) true true "(R=1.000000,G=0.000000,B=0.369439,A=1.000000)" 0.0))
        (:then_1
          (Utilities|FlowControl|DoOnce false
            (:Completed
              (bind _output_get_2 (Variables|Default|SetDefault%20Distance (.Distance (Collision|BreakHitResult _outhit)))))))))
    (:then_1
      (Development|PrintString (Utilities|String|ToString(Float) (Variables|/Script/Engine.CharacterMovementComponent|GetMaxWalkSpeed (Variables|Character|GetCharacterMovement))) true true "(R=0.237480,G=1.000000,B=0.000000,A=1.000000)" 0.0))))

(event Input|KeyboardEvents|V
  (params (Key :type Key%20Structure :default "None"))
  ;[1 0 0] Voice Chat
  (:Pressed
    (Development|ExecuteConsoleCommand "ToggleSpeaking 1" 0))
  (:Released
    (Development|ExecuteConsoleCommand "ToggleSpeaking 0" 0)))

(fn ConstructionScript)
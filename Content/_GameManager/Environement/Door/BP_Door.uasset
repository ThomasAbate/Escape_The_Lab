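; BP_Door is an interactable swinging door that the player toggles open and closed.
; Front and back trigger volumes open gates for the player, letting interaction input through when the player's LookActor is valid.
; The side used sets the swing to plus or minus 90 degrees, and a FlipFlop plays or reverses a timeline that lerps mesh yaw.
; The construction script and CheckThePlayerRun are empty.
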(event OnComponentBeginOverlap(InteractionFront)
  (params (OverlappedComponent :type Primitive%20Component%20Object%20Reference) (OtherActor :type Actor%20Object%20Reference) (OtherComp :type Primitive%20Component%20Object%20Reference) (OtherBodyIndex :type Integer) (bFromSweep :type Boolean) (SweepResult :type Hit%20Result%20Structure%20%28by%20ref%29))
  ;[1 1 1] Normal Open Front
  (if (== OtherActor (Game|GetPlayerCharacter 0))
    (Utilities|FlowControl|Gate true) ; enters at Open
  ))

(event OnComponentBeginOverlap(InteractionBack)
  (params (OverlappedComponent :type Primitive%20Component%20Object%20Reference) (OtherActor :type Actor%20Object%20Reference) (OtherComp :type Primitive%20Component%20Object%20Reference) (OtherBodyIndex :type Integer) (bFromSweep :type Boolean) (SweepResult :type Hit%20Result%20Structure%20%28by%20ref%29))
  ;[1 1 1] Normal Open Back
  (if (== OtherActor (Game|GetPlayerCharacter 0))
    (Utilities|FlowControl|Gate true) ; enters at Open
  ))

(event OnComponentEndOverlap(InteractionFront)
  (params (OverlappedComponent :type Primitive%20Component%20Object%20Reference) (OtherActor :type Actor%20Object%20Reference) (OtherComp :type Primitive%20Component%20Object%20Reference) (OtherBodyIndex :type Integer))
  ;[1 1 1] Normal Open Front
  (if (== (Game|GetPlayerCharacter 0) OtherActor)
    (Utilities|FlowControl|Gate true) ; enters at Close
  ))

(event OnComponentEndOverlap(InteractionBack)
  (params (OverlappedComponent :type Primitive%20Component%20Object%20Reference) (OtherActor :type Actor%20Object%20Reference) (OtherComp :type Primitive%20Component%20Object%20Reference) (OtherBodyIndex :type Integer))
  ;[1 1 1] Normal Open Back
  (if (== (Game|GetPlayerCharacter 0) OtherActor)
    (Utilities|FlowControl|Gate true) ; enters at Close
  ))

(event Custom|Event%20Normal%20Open%20Front
  ;[1 1 1] Open Door / Closs Event
  (Utilities|FlowControl|FlipFlop
    (:A
      (bind _alapha (Timeline|Door%20TimeLine Play)
        (:Update
          (Transformation|SetRelativeRotation (Variables|Default|GetStaticMesh) (Math|Rotator|MakeRotator 0.0 0.0 (Math|Float|Lerp 0.0 (Variables|Default|GetValue%20Of%20Open) _alapha)) false false))))
    (:B
      (Timeline|Door%20TimeLine Reverse))))

(event EventIntractionInput
  (Utilities|FlowControl|Sequence
    (:then_0
      ;[1 1 1] Normal Open Front
      (Utilities|FlowControl|Gate true
        (:Exit
          (Variables|/Game/_GameManager/Player/Blueprints/BP_Player_Charachter.BP_Player_Charachter_C|GetLook%20Actor (.AsBP%20Player%20Charachter (Utilities|Casting|CastToBP_Player_Charachter (Game|GetPlayerCharacter 0)))
            (:then
              (Variables|Default|SetValue%20Of%20Open -9e+01)
              (CallFunction|EventNormalOpenFront))
            (:else)))))
    (:then_1
      ;[1 1 1] Normal Open Back
      (Utilities|FlowControl|Gate true
        (:Exit
          (Variables|/Game/_GameManager/Player/Blueprints/BP_Player_Charachter.BP_Player_Charachter_C|GetLook%20Actor (.AsBP%20Player%20Charachter (Utilities|Casting|CastToBP_Player_Charachter (Game|GetPlayerCharacter 0)))
            (:then
              (Variables|Default|SetValue%20Of%20Open 9e+01)
              (CallFunction|EventNormalOpenFront))
            (:else)))))))

(fn ConstructionScript)

(fn CheckthePlayerRun?)
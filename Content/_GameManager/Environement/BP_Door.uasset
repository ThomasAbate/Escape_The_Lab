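; BP_Door is a physics door that gets knocked open when a running player hits it from either side.
; Overlap triggers Face0 and Face1 check that the actor is BP_Player and that BP_Player_Controller reports running, then apply opposite Y-axis impulses to the DoorWooden component.
; The Face1 push is ten times stronger, both sides print debug strings, and the end-overlap handlers do nothing beyond the player cast.
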(event OnComponentBeginOverlap(Face0)
  (params (OverlappedComponent :type Primitive%20Component%20Object%20Reference) (OtherActor :type Actor%20Object%20Reference) (OtherComp :type Primitive%20Component%20Object%20Reference) (OtherBodyIndex :type Integer) (bFromSweep :type Boolean) (SweepResult :type Hit%20Result%20Structure%20%28by%20ref%29))
  ;[1 1 1] Open The Door when the Player Run
  ;;[1 1 1] Face 1 Door
  ;;;[0.05098 0.05098 0.05098] Open
  (Utilities|Casting|CastToBP_Player OtherActor)
  (if (Variables|/Game/_GameManager/Player/Blueprints/BP_Player_Controller.BP_Player_Controller_C|GetIs%20Runing (.AsBP%20Player%20Controller (Utilities|Casting|CastToBP_Player_Controller (Game|GetPlayerController 0))))
    (Development|PrintString "Hello")
    (Physics|AddImpulse (Variables|Default|GetDoor_Wooden) "0.000000,50000.000000,0.000000" "None" false)))

(event OnComponentEndOverlap(Face0)
  (params (OverlappedComponent :type Primitive%20Component%20Object%20Reference) (OtherActor :type Actor%20Object%20Reference) (OtherComp :type Primitive%20Component%20Object%20Reference) (OtherBodyIndex :type Integer))
  ;[1 1 1] Open The Door when the Player Run
  ;;[1 1 1] Face 1 Door
  ;;;[1 1 1] Closs
  (Utilities|Casting|CastToBP_Player OtherActor))

(event OnComponentBeginOverlap(Face1)
  (params (OverlappedComponent :type Primitive%20Component%20Object%20Reference) (OtherActor :type Actor%20Object%20Reference) (OtherComp :type Primitive%20Component%20Object%20Reference) (OtherBodyIndex :type Integer) (bFromSweep :type Boolean) (SweepResult :type Hit%20Result%20Structure%20%28by%20ref%29))
  ;[1 1 1] Open The Door when the Player Run
  ;;[1 1 1] Face 2 Door
  (Utilities|Casting|CastToBP_Player OtherActor)
  (if (Variables|/Game/_GameManager/Player/Blueprints/BP_Player_Controller.BP_Player_Controller_C|GetIs%20Runing (.AsBP%20Player%20Controller (Utilities|Casting|CastToBP_Player_Controller (Game|GetPlayerController 0))))
    (Development|PrintString "bye")
    (Physics|AddImpulse (Variables|Default|GetDoor_Wooden) "0.000000,-500000.000000,0.000000" "None" false)))

(event OnComponentEndOverlap(Face1)
  (params (OverlappedComponent :type Primitive%20Component%20Object%20Reference) (OtherActor :type Actor%20Object%20Reference) (OtherComp :type Primitive%20Component%20Object%20Reference) (OtherBodyIndex :type Integer))
  ;[1 1 1] Open The Door when the Player Run
  ;;[1 1 1] Face 2 Door
  (Utilities|Casting|CastToBP_Player OtherActor))

(fn ConstructionScript)
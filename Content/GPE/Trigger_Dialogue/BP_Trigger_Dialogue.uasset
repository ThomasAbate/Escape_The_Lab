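; Trigger volume that sends a dialogue message to the player's pawn when it enters the box.
; On overlap, it checks that the other actor is player 0's pawn, then passes DialogueName to SetDialoguesMessage.
; The DoOnce branch leads to an empty completion, so it does not gate repeat messages.
; The construction script sizes the box from the ScaleBox variable.
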(event OnComponentBeginOverlap(Box)
  (params (OverlappedComponent :type Primitive%20Component%20Object%20Reference) (OtherActor :type Actor%20Object%20Reference) (OtherComp :type Primitive%20Component%20Object%20Reference) (OtherBodyIndex :type Integer) (bFromSweep :type Boolean) (SweepResult :type Hit%20Result%20Structure%20%28by%20ref%29))
  (bind _returnvalue (Game|Player|GetPlayerPawn 0))
  (if (Variables|Components|GetDo%20once)
    (Utilities|FlowControl|DoOnce false
      (:Completed
        _)))
  (if (== OtherActor _returnvalue)
    (Class|BPIDialogue|SetDialogues(Message) _returnvalue (Variables|Dialogue|GetDialogue_Name))))

(event EventBeginPlay)

(fn ConstructionScript
  (Components|Box|SetBoxExtent (Variables|Default|GetBox) (Variables|Components|GetScale_Box) true))
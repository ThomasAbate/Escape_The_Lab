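; Elevator actor whose double sliding doors open on request and close behind the player.
; Its ToDo event triggers opening, which plays a sound, arms closing and runs a timeline that lerps both door meshes apart.
; When the player pawn overlaps the trigger while armed, it disarms, plays the closing sound and reverses the same timeline.
; The file contains only door logic, with no cabin movement.
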(event OnComponentBeginOverlap(TriggerToCloos_0)
  (params (OverlappedComponent :type Primitive%20Component%20Object%20Reference) (OtherActor :type Actor%20Object%20Reference) (OtherComp :type Primitive%20Component%20Object%20Reference) (OtherBodyIndex :type Integer) (bFromSweep :type Boolean) (SweepResult :type Hit%20Result%20Structure%20%28by%20ref%29))
  (if (and (== OtherActor (Game|Player|GetPlayerPawn 0)) (Variables|Default|GetCan%20Be%20Cloos))
    (CallFunction|EventCloseDoor)))

(event Custom|Event%20Open%20Door
  (Audio|PlaySoundatLocation "/Game/Audio/Elevator/A_Elevator_Door_Open.A_Elevator_Door_Open" (Transformation|GetActorLocation) "0, 0, 0" 1.0 1.0 0.0 0 0 0 0)
  (Variables|Default|SetCan%20Be%20Cloos true)
  (bind _alpha (Timeline|Alpha%20Door%20Anim Play)
    (:Update
      (Transformation|SetRelativeLocation (Variables|Default|GetSM_Door_Elevator_R) (Math|Vector|Lerp(Vector) "75.000000,150.000000,25.000000" "110.000000,150.000000,25.000000" _alpha) false false)
      (Transformation|SetRelativeLocation (Variables|Default|GetSM_Door_Elevator_L) (Math|Vector|Lerp(Vector) "-75.000000,150.000000,25.000000" "-110.000000,150.000000,25.000000" _alpha) false false))))

(event Custom|Event%20Close%20Door
  (Audio|PlaySoundatLocation "/Game/Audio/Elevator/A_Elevator_Door_Close.A_Elevator_Door_Close" (Transformation|GetActorLocation) "0, 0, 0" 1.0 1.0 0.0 0 0 0 0)
  (Variables|Default|SetCan%20Be%20Cloos false)
  (bind _alpha (Timeline|Alpha%20Door%20Anim Reverse)
    (:Update
      (Transformation|SetRelativeLocation (Variables|Default|GetSM_Door_Elevator_R) (Math|Vector|Lerp(Vector) "75.000000,150.000000,25.000000" "110.000000,150.000000,25.000000" _alpha) false false)
      (Transformation|SetRelativeLocation (Variables|Default|GetSM_Door_Elevator_L) (Math|Vector|Lerp(Vector) "-75.000000,150.000000,25.000000" "-110.000000,150.000000,25.000000" _alpha) false false))))

(event EventToDo
  (CallFunction|EventOpenDoor))

(fn ConstructionScript)
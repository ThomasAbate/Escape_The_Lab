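; BP_Puzzel_001 is a possessable puzzle object that the player takes control of to rotate its mesh.
; On interaction it fades the camera out, possesses itself and fades back in; look input then spins the mesh, and the interact input returns control to the stored player with the same fade.
; When UnlockActor is set, UnlockObject flip-flops between an empty, non-triggerable state and a visible, triggerable one, starting empty on BeginPlay.
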(event Input|EnhancedActionEvents|EnhancedInputActionIA_Look
  (params (ActionValue :type Vector%202D%20Structure) (ElapsedSeconds :type Float%20%28double-precision%29) (TriggeredSeconds :type Float%20%28double-precision%29) (InputAction :type Input%20Action%20Object%20Reference :default "/Game/ThirdPerson/Input/Actions/IA_Look.IA_Look"))
  (bind (_x _y) (Math|Vector2D|BreakVector2D ActionValue))
  (bind _output_get (Variables|Default|SetX _x))
  (bind _output_get_2 (Variables|Default|SetY _y))
  (Transformation|AddLocalRotation (Variables|Default|GetStaticMesh) (Math|Rotator|MakeRotator _output_get _output_get_2 0.0) false false))

(event Input|EnhancedActionEvents|EnhancedInputActionIA_Interaction
  (params (ActionValue :type Boolean) (ElapsedSeconds :type Float%20%28double-precision%29) (TriggeredSeconds :type Float%20%28double-precision%29) (InputAction :type Input%20Action%20Object%20Reference :default "/Game/ThirdPerson/Input/Actions/IA_Interaction.IA_Interaction"))
  (CameraFades|StartCameraFade :self (Game|GetPlayerCameraManager 0) :ToAlpha 1.0 :Duration 0.5 :bHoldWhenFinished true)
  (Utilities|FlowControl|Delay 0.55)
  (Pawn|Possess (Game|GetPlayerController 0) (Variables|Default|GetPlayer))
  (Collision|SetCollisionEnabled (Variables|Default|GetStaticMesh) "QueryAndPhysics")
  (Class|BPIObjectPosses|SetPlayerVisibility(Message) (Variables|Default|GetPlayer) true)
  (CameraFades|StartCameraFade :self (Game|GetPlayerCameraManager 0) :FromAlpha 1.0 :Duration 0.5))

(event EventUnlockObject
  (bind _trigger_box (Variables|Default|GetTrigger%20Box))
  (bind _staticmesh (Variables|Default|GetStaticMesh))
  (if (Variables|Default|GetUnlock%20Actor)
    (Utilities|FlowControl|FlipFlop
      (:A
        (Components|StaticMesh|SetStaticMesh _staticmesh 0)
        (Collision|SetCollisionEnabled _trigger_box "NoCollision"))
      (:B
        (Components|StaticMesh|SetStaticMesh _staticmesh (Variables|Default|GetObject))
        (Collision|SetCollisionEnabled _trigger_box "QueryOnly")))))

(event EventBeginPlay
  (CallFunction|UnlockObject))

(event EventUpdateItemInteracted
  (params (Pawn :type Pawn%20Object%20Reference))
  (CallFunction|Enter Pawn)
  (Class|BPIObjectPosses|SetPlayerVisibility(Message) (Game|Player|GetPlayerPawn 0) false))

(event EventEnter
  (params (Player :type Pawn%20Object%20Reference))
  (CameraFades|StartCameraFade :self (Game|GetPlayerCameraManager 0) :ToAlpha 1.0 :Duration 0.5 :bHoldWhenFinished true)
  (Utilities|FlowControl|Delay 0.55)
  (Pawn|Possess (Game|GetPlayerController 0) self)
  (bind _output_get (Variables|Default|SetPlayer Player))
  (Class|BPIObjectPosses|SetPlayerVisibility(Message) _output_get false)
  (Collision|SetCollisionEnabled (Variables|Default|GetStaticMesh) "NoCollision")
  (CameraFades|StartCameraFade :self (Game|GetPlayerCameraManager 0) :FromAlpha 1.0 :Duration 0.5))

(fn ConstructionScript
  (|CallParentFunction))
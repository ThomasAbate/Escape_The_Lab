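; Base interactable object that sets its mesh and trigger box size at construction and reacts to player interaction.
; Trigger overlaps set the mesh overlay material and open or close a gate on the interaction effects.
; Interaction disables or toggles mesh collision, even outside the gate.
; Through the gate, it plays a pickup sound, calls an empty item-update hook, and optionally starts dialogue or sends a look-at-object message to the player.
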(event OnComponentBeginOverlap(TriggerBox)
  (params (OverlappedComponent :type Primitive%20Component%20Object%20Reference) (OtherActor :type Actor%20Object%20Reference) (OtherComp :type Primitive%20Component%20Object%20Reference) (OtherBodyIndex :type Integer) (bFromSweep :type Boolean) (SweepResult :type Hit%20Result%20Structure%20%28by%20ref%29))
  (bind _look_object (Variables|Look|GetLook%20Object))
  ;[1 1 1] Check the player can interact
  (if (== OtherActor (Game|Player|GetPlayerPawn 0))
    (Variables|/Game/ThirdPerson/Blueprints/Player/BP_ThirdPersonCharacter.BP_ThirdPersonCharacter_C|SetIs%20range%20? (Variables|Components|GetAs%20BP%20Third%20Person%20Character) true)
    (Rendering|Material|SetOverlayMaterial (Variables|Default|GetStaticMesh) 0 :!class /Script/Engine.MeshComponent)
    (Utilities|FlowControl|Gate true) ; enters at Open
  ))

(event OnComponentEndOverlap(TriggerBox)
  (params (OverlappedComponent :type Primitive%20Component%20Object%20Reference) (OtherActor :type Actor%20Object%20Reference) (OtherComp :type Primitive%20Component%20Object%20Reference) (OtherBodyIndex :type Integer))
  (bind _look_object (Variables|Look|GetLook%20Object))
  ;[1 1 1] Check the player can interact
  (if (== (Game|Player|GetPlayerPawn 0) OtherActor)
    (Variables|/Game/ThirdPerson/Blueprints/Player/BP_ThirdPersonCharacter.BP_ThirdPersonCharacter_C|SetIs%20range%20? (Variables|Components|GetAs%20BP%20Third%20Person%20Character) true)
    (Rendering|Material|SetOverlayMaterial (Variables|Default|GetStaticMesh) 0 :!class /Script/Engine.MeshComponent)
    (Utilities|FlowControl|Gate true) ; enters at Close
  ))

(event Custom|Update%20Item%20interacted
  (params (Pawn :type Pawn%20Object%20Reference)))

(event EventBeginPlay
  (bind _asbp_third_person_character (Utilities|Casting|CastToBP_ThirdPersonCharacter (Game|Player|GetPlayerPawn 0)))
  (Variables|Components|SetAs%20BP%20Third%20Person%20Character _asbp_third_person_character))

(event EventInteraction
  (bind _look_object (Variables|Look|GetLook%20Object))
  ;[1 1 1] Check the player can interact
  (if (Variables|OnSpawn|GetDo%20Once)
    (Collision|SetCollisionEnabled (Variables|Default|GetStaticMesh) "NoCollision" :!label _label)
    (else
      (Utilities|FlowControl|FlipFlop
        (:A
          (goto _label))
        (:B
          (Collision|SetCollisionEnabled (Variables|Default|GetStaticMesh) "QueryAndPhysics")))))
  (Utilities|FlowControl|Gate true
    (:Exit
      (Audio|PlaySound2D (Variables|Sound|GetSound%20Take%20Object) 1.0 1.0 0.0 0 0)
      (Utilities|FlowControl|Sequence
        (:then_0
          (CallFunction|UpdateItemInteracted (Game|Player|GetPlayerPawn 0)))
        (:then_1
          (if (Variables|Talk|GetNeed%20To%20Talk)
            (Utilities|FlowControl|Delay 0.2)
            (Default|EventForceDeleteDialogue (Variables|/Game/ThirdPerson/Blueprints/Player/BP_ThirdPersonCharacter.BP_ThirdPersonCharacter_C|GetBPC_Dialogue (Variables|Components|GetAs%20BP%20Third%20Person%20Character)))
            (Utilities|FlowControl|DelayUntilNextTick)
            (Variables|/Game/ThirdPerson/Blueprints/Player/BP_ThirdPersonCharacter.BP_ThirdPersonCharacter_C|SetCan%20Talk%20? (Variables|Components|GetAs%20BP%20Third%20Person%20Character) true)
            (Class|BPIDialogue|SetDialogues(Message) (Game|Player|GetPlayerPawn 0) (Variables|Talk|GetDialogue))))
        (:then_2
          (if _look_object
            (Class|BPIInteraction|ToLook(Message) (Game|Player|GetPlayerPawn 0) (Variables|OnSpawn|GetObject) (Variables|Look|GetDistance) _look_object)))))))

(fn ConstructionScript
  (Components|StaticMesh|SetStaticMesh (Variables|Default|GetStaticMesh) (Variables|OnSpawn|GetObject))
  (Components|Box|SetBoxExtent (Variables|Default|GetTrigger%20Box) (Variables|OnSpawn|GetIn%20Box%20Extent) true))
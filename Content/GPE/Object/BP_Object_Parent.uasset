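; Parent Blueprint for world objects the player can take, with mesh and trigger size set per instance in the construction script.
; The trigger box opens a gate while the player overlaps, letting Interaction play a sound, print the name and disable mesh collision.
; It then calls UpdateItemWhenIsTaken, an empty hook likely meant for children.
; If NeedToTalk is set, it clears current dialogue and shows its own through the player character.
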(event OnComponentBeginOverlap(TriggerBox)
  (params (OverlappedComponent :type Primitive%20Component%20Object%20Reference) (OtherActor :type Actor%20Object%20Reference) (OtherComp :type Primitive%20Component%20Object%20Reference) (OtherBodyIndex :type Integer) (bFromSweep :type Boolean) (SweepResult :type Hit%20Result%20Structure%20%28by%20ref%29))
  (bind _as_bp_third_person_character (Variables|Components|GetAs%20BP%20Third%20Person%20Character))
  (if (== OtherActor (Game|Player|GetPlayerPawn 0))
    (Utilities|FlowControl|Gate true) ; enters at Open
  ))

(event OnComponentEndOverlap(TriggerBox)
  (params (OverlappedComponent :type Primitive%20Component%20Object%20Reference) (OtherActor :type Actor%20Object%20Reference) (OtherComp :type Primitive%20Component%20Object%20Reference) (OtherBodyIndex :type Integer))
  (bind _as_bp_third_person_character (Variables|Components|GetAs%20BP%20Third%20Person%20Character))
  (if (== (Game|Player|GetPlayerPawn 0) OtherActor)
    (Utilities|FlowControl|Gate true) ; enters at Close
  ))

(event Custom|Event%20Update%20Item%20When%20is%20taken)

(event EventBeginPlay
  (bind _asbp_third_person_character (Utilities|Casting|CastToBP_ThirdPersonCharacter (Game|Player|GetPlayerPawn 0)))
  (Variables|Components|SetAs%20BP%20Third%20Person%20Character _asbp_third_person_character))

(event EventInteraction
  (bind _as_bp_third_person_character (Variables|Components|GetAs%20BP%20Third%20Person%20Character))
  (Utilities|FlowControl|Gate true
    (:Exit
      (Audio|PlaySound2D (Variables|Sound|GetSound%20Take%20Object) 1.0 1.0 0.0 0 0)
      (Development|PrintString (Utilities|String|Append (Utilities|GetDisplayName self) " Taken"))
      (Collision|SetCollisionEnabled (Variables|Default|GetStaticMesh) "NoCollision")
      (Utilities|FlowControl|Sequence
        (:then_0
          (CallFunction|EventUpdateItemwhenIsTaken))
        (:then_1
          (if (Variables|Talk|GetNeed%20To%20Talk)
            (Utilities|FlowControl|Delay 0.2)
            (Default|EventForceDeleteDialogue (Variables|/Game/ThirdPerson/Blueprints/Player/BP_ThirdPersonCharacter.BP_ThirdPersonCharacter_C|GetBPC_Dialogue (Variables|Components|GetAs%20BP%20Third%20Person%20Character)))
            (Utilities|FlowControl|DelayUntilNextTick)
            (Variables|/Game/ThirdPerson/Blueprints/Player/BP_ThirdPersonCharacter.BP_ThirdPersonCharacter_C|SetCan%20Talk%20? _as_bp_third_person_character true)
            (Class|BPIDialogue|SetDialogues(Message) _as_bp_third_person_character (Variables|Talk|GetDialogue))))))))

(fn ConstructionScript
  (Components|StaticMesh|SetStaticMesh (Variables|Default|GetStaticMesh) (Variables|OnSpawn|GetObject))
  (Components|Box|SetBoxExtent (Variables|Default|GetTrigger%20Box) (Variables|OnSpawn|GetIn%20Box%20Extent) true))
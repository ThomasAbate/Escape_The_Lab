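; BP_BagPack is a backpack item that shrinks away when taken and can notify the level's elevator.
; On BeginPlay it finds and caches a BP_Elevator actor.
; UpdateItemwhenIsTaken plays a timeline that scales the static mesh from full size to zero.
; When the timeline finishes, it calls ToDoMessage on the elevator if DoSomething is set, then destroys itself.
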(event EventBeginPlay
  (bind _returnvalue (Actor|GetActorOfClass "/Game/GPE/Elevator/BP_Elevator.BP_Elevator_C"))
  (Variables|Default|SetElevator _returnvalue))

(event EventUpdateItemwhenIsTaken
  (bind _alpha (Timeline|Timeline Play)
    (:Update
      (Variables|Default|SetAlpha%20Anim _alpha)
      (Transformation|SetRelativeScale3D (Variables|Default|GetStaticMesh) (Math|Vector|Lerp(Vector) "1.000000,1.000000,1.000000" "0, 0, 0" (Variables|Default|GetAlpha%20Anim))))
    (:Finished
      (if (Variables|Default|GetDo%20something%20?)
        (Class|BPIInteraction|ToDo(Message) (Variables|Default|GetElevator)))
      (Actor|DestroyActor))))

(fn ConstructionScript
  (|CallParentFunction))
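; BP_Car is an interactable car object that either ends the current level or sets off an alarm when taken.
; If it is flagged as the player's car, it fades the camera out, locks movement and look input, then loads LVL_Main after a short delay.
; Otherwise it plays a car alarm sound at the mesh's location.
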(event EventUpdateItemwhenIsTaken
  (bind _returnvalue (Game|GetPlayerController 0))
  (if (Variables|Car|GetYour%20Car)
    (CameraFades|StartCameraFade :self (Game|GetPlayerCameraManager 0) :ToAlpha 1.0 :Duration 3.0 :bHoldWhenFinished true)
    (Input|SetIgnoreMoveInput _returnvalue true)
    (Input|SetIgnoreLookInput _returnvalue true)
    (Utilities|FlowControl|Delay 3.0)
    (Game|OpenLevel(byObjectReference) "/Game/Level/LVL_Main.LVL_Main")
    (else
      (Audio|PlaySoundatLocation "/Game/Audio/A_Car_alarm.A_Car_alarm" (Transformation|GetWorldLocation (Variables|Default|GetStaticMesh)) "0, 0, 0" 1.0 1.0 0.0 0 0 0 0))))

(fn ConstructionScript
  (|CallParentFunction))
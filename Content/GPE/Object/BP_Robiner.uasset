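; BP_Robiner is an interactive object, apparently a faucet, that toggles the display of running water.
; It hides its WaterPlane and Water components on BeginPlay.
; Each UpdateItemwhenIsTaken event alternately shows and hides both components through a FlipFlop.
; The construction script only calls the parent's.
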(event EventUpdateItemwhenIsTaken
  (Utilities|FlowControl|FlipFlop
    (:A
      (Rendering|SetVisibility (Variables|Default|GetWater_Plane) true false)
      (Rendering|SetVisibility (Variables|Default|GetWater) true false))
    (:B
      (Rendering|SetVisibility (Variables|Default|GetWater_Plane) false false)
      (Rendering|SetVisibility (Variables|Default|GetWater) false false))))

(event EventBeginPlay
  (Rendering|SetVisibility (Variables|Default|GetWater_Plane) false false)
  (Rendering|SetVisibility (Variables|Default|GetWater) false false))

(fn ConstructionScript
  (|CallParentFunction))